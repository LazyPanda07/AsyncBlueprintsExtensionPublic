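; BP_InfiniteTask is an async task Blueprint from AsyncBlueprintsExtension that measures actor distances to a Character reference.
; Initialization caches every Actor in the world once.
; Execute loops over that cache, overwriting LastCalculated with each distance, so only the final actor's distance gets printed.
; It then waits a second, with no repeat loop in the graph itself despite the "Infinite" name.
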(event EventExecute
  (for _array_element (Variables|Default|GetActors)
    (Variables|Default|SetLastCalculated (Math|Vector|VectorLength (- (Transformation|GetActorLocation _array_element) (Transformation|GetActorLocation (Variables|Default|GetCharacter))))))
  (Development|PrintString (Utilities|String|ToString(Float) (Variables|Default|GetLastCalculated)))
  (Class|AsyncLibrary|Wait 1.0))

(event EventInitialization
  (bind _outactors (Actor|GetAllActorsOfClass "/Script/Engine.Actor"))
  (Variables|Default|SetActors _outactors))